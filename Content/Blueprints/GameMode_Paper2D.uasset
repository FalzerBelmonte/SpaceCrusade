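; Game mode for a Paper2D character game that adds the HUD and handles player damage, death and respawn.
; PlayerHurt lowers health with a brief scale and tint flash, sound and camera shake, destroying the player and calling Respawn when health runs out.
; Respawn shows a countdown widget, spawns BP_Spawner at the checkpoint and disables movement for three seconds before restoring flying.
; Tick also disables movement once while health is depleted.
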(event Custom|PlayerHurt
  (params (Player :type Actor%20Object%20Reference))
  (bind _aspaper_2d_character (Utilities|Casting|CastToPaper2D_Character Player))
  (bind _healthcheck (CallFunction|DamageAnimation Player))
  (Utilities|FlowControl|Delay 0.15)
  (Transformation|SetActorRelativeScale3D _aspaper_2d_character "1.000000,1.000000,1.000000")
  (Sprite|SetSpriteColor (Variables|/Script/Paper2D.PaperCharacter|GetSprite _aspaper_2d_character) (- "(R=1.000000,G=1.000000,B=1.000000,A=1.000000)" ""))
  (if (not _healthcheck)
    (Actor|DestroyActor Player)
    (Utilities|Respawn)))

(event EventBeginPlay
  (bind _returnvalue (UserInterface|CreateWidget "/Game/Widgets/WBP_HUD.WBP_HUD_C"))
  (UserInterface|Viewport|AddtoViewport _returnvalue 0))

(event EventTick
  (params (DeltaSeconds :type Float%20%28single-precision%29))
  (bind _aspaper_2d_character (Utilities|Casting|CastToPaper2D_Character (Game|GetPlayerCharacter 0)))
  (Variables|Default|SetSpawner _aspaper_2d_character)
  (if (<= (Variables|/Game/Blueprints/Characters/Paper2D_Character.Paper2D_Character_C|GetHealth _aspaper_2d_character) 0.0)
    (Utilities|FlowControl|DoOnce false :!label _label
      (:Completed
        (bind _aspaper_2d_character_2 (Utilities|Casting|CastToPaper2D_Character (Game|GetPlayerCharacter 0)))
        (Pawn|Components|CharacterMovement|SetMovementMode (Variables|/Script/Engine.Character|GetCharacterMovement _aspaper_2d_character_2) "MOVE_None" 0)))
    (else
      (goto _label Reset))))

(fn ConstructionScript)

(fn DamageAnimation
  (params (PlayerInput :type Actor%20Object%20Reference))
  (bind _aspaper_2d_character (Utilities|Casting|CastToPaper2D_Character PlayerInput))
  (bind _output_get (Variables|/Game/Blueprints/Characters/Paper2D_Character.Paper2D_Character_C|SetHealth _aspaper_2d_character (- (Variables|/Game/Blueprints/Characters/Paper2D_Character.Paper2D_Character_C|GetHealth _aspaper_2d_character) 0.1)))
  (Audio|SpawnSoundatLocation "/Game/AudioFile/SpikeSounds.SpikeSounds" "0, 0, 0" "0, 0, 0" 1.0 1.0 0.0 0 0)
  (Transformation|SetActorRelativeScale3D _aspaper_2d_character "1.100000,1.100000,1.200000")
  (Sprite|SetSpriteColor (Variables|/Script/Paper2D.PaperCharacter|GetSprite _aspaper_2d_character) (+ "(R=0.640625,G=0.150146,B=0.150146,A=1.000000)" ""))
  (Camera|PlayWorldCameraShake "/Game/Blueprints/Camera/BP_CameraShake.BP_CameraShake_C" (Transformation|GetActorLocation _aspaper_2d_character) 3e+03 5e+02 5.0)
  (return 0 (> _output_get 0.0)))

(fn TimerDown
  (Utilities|Casting|CastToPaper2D_Character (Game|GetPlayerCharacter 0))
  (bind _returnvalue (UserInterface|CreateWidget "/Game/Widgets/WBP_CountDown.WBP_CountDown_C"))
  (bind _returnvalue_2 (UserInterface|Animation|PlayAnimation _returnvalue (Variables|Default|GetCountdown) 0.0 1 "Forward" 1.0 false))
  (return _returnvalue_2))