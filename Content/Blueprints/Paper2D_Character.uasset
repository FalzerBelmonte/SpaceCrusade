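; Paper2D character Blueprint for a player moving on fixed world axes, with an eight-direction flipbook sprite.
; X and Y axis inputs drive movement, and each tick SetDirection derives a facing from them, keeping the last one without input.
; The facing selects the flipbook; moving and stationary branches both use the same idle flipbooks.
; The construction script tilts the sprite using the spring arm's pitch.
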(event EventTick
  (params (DeltaSeconds :type Float%20%28single-precision%29))
  (CallFunction|SetDirection))

(event Input|AxisEvents|InputAxisXAxis
  (params (AxisValue :type Float%20%28single-precision%29))
  (Pawn|Input|AddMovementInput "0.000000,-1.000000, 0" AxisValue true))

(event Input|AxisEvents|InputAxisYAxis
  (params (AxisValue :type Float%20%28single-precision%29))
  (Pawn|Input|AddMovementInput "-1.000000,0.000000, 0" AxisValue true))

(fn ConstructionScript
  (Transformation|SetWorldRotation (Variables|Default|GetSprite) (Math|Rotator|MakeRotator (.pitch (Transformation|GetWorldRotation (Variables|Camera|GetSpringArm))) 0.0 -9e+01) false false))

(fn SetDirection
  (if (or (!= (Input|AxisValues|GetXAxis) 0.0) (!= (Input|AxisValues|GetYAxis) 0.0))
    (Variables|Default|SetDirection (select (and (> (Input|AxisValues|GetXAxis) 0.0) (> (Input|AxisValues|GetYAxis) 0.0)) "NewEnumerator4" (select (and (< (Input|AxisValues|GetXAxis) 0.0) (< (Input|AxisValues|GetYAxis) 0.0)) "NewEnumerator7" (select (and (> (Input|AxisValues|GetXAxis) 0.0) (< (Input|AxisValues|GetYAxis) 0.0)) "NewEnumerator6" (select (and (< (Input|AxisValues|GetXAxis) 0.0) (> (Input|AxisValues|GetYAxis) 0.0)) "NewEnumerator5" (select (> (Input|AxisValues|GetYAxis) 0.0) "NewEnumerator0" (select (< (Input|AxisValues|GetYAxis) 0.0) "NewEnumerator1" (select (> (Input|AxisValues|GetXAxis) 0.0) "NewEnumerator2" "NewEnumerator3"))))))))
    (Sprite|SetFlipbook (Variables|Default|GetSprite) (select (> (Math|Vector|VectorLength (Transformation|GetVelocity)) 0.0) (Utilities|Select :Index (Variables|Default|GetDirection) :NewEnumerator0 "/Game/Sprites/Character/FB_UpIdle.FB_UpIdle" :NewEnumerator1 "/Game/Sprites/Character/FB_DownIdle.FB_DownIdle" :NewEnumerator2 "/Game/Sprites/Character/FB_RightIdle.FB_RightIdle" :NewEnumerator3 "/Game/Sprites/Character/FB_LeftIdle.FB_LeftIdle" :NewEnumerator4 "/Game/Sprites/Character/FB_NEastIdle.FB_NEastIdle" :NewEnumerator5 "/Game/Sprites/Character/FB_NWestIdle.FB_NWestIdle" :NewEnumerator6 "/Game/Sprites/Character/FB_SEastIdle.FB_SEastIdle" :NewEnumerator7 "/Game/Sprites/Character/FB_SWestIdle.FB_SWestIdle") (Utilities|Select :Index (Variables|Default|GetDirection) :NewEnumerator0 "/Game/Sprites/Character/FB_UpIdle.FB_UpIdle" :NewEnumerator1 "/Game/Sprites/Character/FB_DownIdle.FB_DownIdle" :NewEnumerator2 "/Game/Sprites/Character/FB_RightIdle.FB_RightIdle" :NewEnumerator3 "/Game/Sprites/Character/FB_LeftIdle.FB_LeftIdle" :NewEnumerator4 "/Game/Sprites/Character/FB_NEastIdle.FB_NEastIdle" :NewEnumerator5 "/Game/Sprites/Character/FB_NWestIdle.FB_NWestIdle" :NewEnumerator6 "/Game/Sprites/Character/FB_SEastIdle.FB_SEastIdle" :NewEnumerator7 "/Game/Sprites/Character/FB_SWestIdle.FB_SWestIdle")))))