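; Game instance Blueprint that sets up the player's save data when it initializes.
; On Init it checks the save slot and either calls LoadGame or creates a new BP_PlayerSaveData object in memory.
; LoadGame reads the slot and casts the result to BP_PlayerSaveData.
; Both paths store the object in SaveGameData; nothing here writes it back to disk.
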(event EventInit
  (bind _returnvalue (SaveGame|DoesSaveGameExist (Variables|Default|GetSaveGameSlot)))
  (if _returnvalue
    (CallFunction|LoadGame)
    (else
      (bind _returnvalue_2 (SaveGame|CreateSaveGameObject "/Game/Blueprints/SaveData/BP_PlayerSaveData.BP_PlayerSaveData_C"))
      (Variables|Default|SetSaveGameData _returnvalue_2))))

(fn LoadGame
  (bind _returnvalue (SaveGame|LoadGamefromSlot (Variables|Default|GetSaveGameSlot)))
  (bind _asbp_player_save_data (Utilities|Casting|CastToBP_PlayerSaveData _returnvalue))
  (Variables|Default|SetSaveGameData _asbp_player_save_data)
  (return))