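; BP_Checkpoint is a checkpoint trigger that records the player's location in a save game.
; Any overlap with its Box reads player 0's Paper2D_Character location and prints a confirmation.
; It then writes that location to a BP_SaveRespawn in slot "check", loading the existing save or creating one.
; The existing-save branch calls SaveGameToSlot without the loaded object connected, unlike the new-save branch.
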(event OnComponentBeginOverlap(Box)
  (params (OverlappedComponent :type Primitive%20Component%20Object%20Reference) (OtherActor :type Actor%20Object%20Reference) (OtherComp :type Primitive%20Component%20Object%20Reference) (OtherBodyIndex :type Integer) (bFromSweep :type Boolean) (SweepResult :type Hit%20Result%20Structure%20%28by%20ref%29))
  (Utilities|FlowControl|Sequence
    (:then_0
      (bind _aspaper_2d_character (Utilities|Casting|CastToPaper2D_Character (Game|GetPlayerCharacter 0)))
      (Variables|Default|SetPlayerLocation (Transformation|GetActorLocation _aspaper_2d_character))
      (Development|PrintString "Checkpoint Reached"))
    (:then_1
      (bind _returnvalue (SaveGame|DoesSaveGameExist "check"))
      (if _returnvalue
        (bind _returnvalue_2 (SaveGame|LoadGamefromSlot "check"))
        (bind _asbp_save_respawn (Utilities|Casting|CastToBP_SaveRespawn _returnvalue_2))
        (Variables|/Game/Blueprints/Checkpoint/BP_SaveRespawn.BP_SaveRespawn_C|SetPlayer_Location _asbp_save_respawn (Variables|Default|GetPlayerLocation))
        (SaveGame|SaveGametoSlot 0 "check")
        (else
          (bind _returnvalue_3 (SaveGame|CreateSaveGameObject "/Game/Blueprints/Checkpoint/BP_SaveRespawn.BP_SaveRespawn_C"))
          (Variables|/Game/Blueprints/Checkpoint/BP_SaveRespawn.BP_SaveRespawn_C|SetPlayer_Location _returnvalue_3 (Variables|Default|GetPlayerLocation))
          (SaveGame|SaveGametoSlot _returnvalue_3 "check"))))))

(fn ConstructionScript)