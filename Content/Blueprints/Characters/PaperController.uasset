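; PaperController is a controller Blueprint that tracks player experience and level and shows them on the HUD.
; On BeginPlay it creates the WBP_HUD widget for the first player controller and adds it to the viewport.
; AddXP accumulates experience and either updates the HUD progress ratio or triggers LevelUp.
; LevelUp resets experience without carrying overflow, grows the next threshold by a percentage, increments the level and refreshes the HUD.
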(event Custom|LevelUp
  (bind _playerui (Variables|Default|GetPlayerUI))
  (Variables|Default|SetCurrentXP 0.0)
  (Variables|Default|SetMaxLevelXP (+ (Variables|Default|GetMaxLevelXP) (* (Variables|Default|GetMaxLevelXP) 0.15)))
  (Variables|Default|SetPlayerLevel (+ (Variables|Default|GetPlayerLevel) 1))
  (Default|AddXPtoUI _playerui 0.0)
  (Default|LevelUPUI _playerui (Variables|Default|GetPlayerLevel)))

(event EventBeginPlay
  (bind _returnvalue (UserInterface|CreateWidget "/Game/Widgets/WBP_HUD.WBP_HUD_C" (Game|GetPlayerController 0)))
  (bind _output_get (Variables|Default|SetPlayerUI _returnvalue))
  (UserInterface|Viewport|AddtoViewport _output_get 0))

(event EventAddXP
  (params (IncomingXP :type Float%20%28single-precision%29))
  (bind _output_get (Variables|Default|SetCurrentXP (+ (Variables|Default|GetCurrentXP) IncomingXP)))
  (if (>= (/ _output_get (Variables|Default|GetMaxLevelXP)) 1.0)
    (CallFunction|LevelUp)
    (else
      (Default|AddXPtoUI (Variables|Default|GetPlayerUI) (/ _output_get (Variables|Default|GetMaxLevelXP))))))

(fn ConstructionScript)