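; Player-controlled Paper2D character with eight-direction walk and idle flipbooks, sword attacks and a pause menu.
; Tick turns SpringArm1 toward the cursor's hit point and picks the flipbook from input direction and velocity.
; Attacking spawns S_Sword at Arrow1 with the same cursor-facing yaw.
; BeginPlay tints the sprite through a dynamic material using the game instance's loaded highlight colour, while E toggles pause, menu widget and input mode.
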(event Custom|PauseUnpauseGame
  (bind _returnvalue (Game|GetPlayerController 0))
  (bind _gameinstancereference (Variables|Default|GetGameInstanceReference))
  ;[1 1 1] Pause Menu
  (bind _output_get (Variables|/Game/Blueprints/SaveData/BP_SaveGameInstance.BP_SaveGameInstance_C|SetbIsGamePaused _gameinstancereference (not (Variables|/Game/Blueprints/SaveData/BP_SaveGameInstance.BP_SaveGameInstance_C|GetbIsGamePaused _gameinstancereference))))
  (Game|SetGamePaused _output_get)
  (if _output_get
    (bind _returnvalue_2 (UserInterface|CreateWidget "/Game/Widgets/WBP_PauseMenu.WBP_PauseMenu_C"))
    (bind _output_get_2 (Variables|Default|SetPauseMenuReference _returnvalue_2))
    (UserInterface|Viewport|AddtoViewport _output_get_2 0)
    (EventDispatchers|BindEventtoPauseUnpauseEventDispatcher _output_get_2 (delegate Custom|PauseUnpauseGame))
    (Input|SetInputModeGameandUI _returnvalue (Variables|Default|GetPauseMenuReference) "DoNotLock" false)
    (Variables|/Script/Engine.PlayerController|SetbShowMouseCursor _returnvalue true)
    (elif (Utilities|IsValid (Variables|Default|GetPauseMenuReference))
      (Widget|RemovefromParent (Variables|Default|GetPauseMenuReference))
      (Variables|Default|SetPauseMenuReference 0)
      (Input|SetInputModeGameOnly _returnvalue)
      (Variables|/Script/Engine.PlayerController|SetbShowMouseCursor _returnvalue false))))

(event EventBeginPlay
  ;[1 1 1] CharacterCustomizedColor
  (Variables|Default|SetCurrentSwing 0)
  (bind _returnvalue (Rendering|Material|CreateDynamicMaterialInstance (Variables|Default|GetSprite) 0 "/Game/Materials/Int_Cosmestic_Color.Int_Cosmestic_Color" "None" :!class /Script/Engine.PrimitiveComponent))
  (Variables|Default|SetDynamicColourInstance _returnvalue)
  (bind _asbp_save_game_instance (Utilities|Casting|CastToBP_SaveGameInstance (Game|GetGameInstance)))
  (bind _output_get (Variables|Default|SetGameInstanceReference _asbp_save_game_instance))
  (Rendering|Material|SetVectorParameterValue (Variables|Default|GetDynamicColourInstance) "Base Colour" (.highlightcolour (Variables|/Game/Blueprints/SaveData/BP_SaveGameInstance.BP_SaveGameInstance_C|GetLoadedCharacter _output_get)) :!class /Script/Engine.MaterialInstanceDynamic))

(event EventTick
  (params (DeltaSeconds :type Float%20%28single-precision%29))
  ;[1 1 1] Weapon Rotation and set the character's walking animation
  (Utilities|FlowControl|Sequence
    (:then_0
      (Transformation|SetWorldRotation (Variables|Default|GetSpringArm1) (Math|Rotator|MakeRotator 9e+01 (.roll (Transformation|GetActorRotation)) (+ (.yaw (Math|Rotator|FindLookatRotation (Transformation|GetActorLocation) (.Location (Collision|BreakHitResult (.HitResult (Game|Player|GetHitResultUnderCursorbyChannel (Game|GetPlayerController 0) "TraceTypeQuery1" true)))))) -1.8e+02)) false false))
    (:then_1
      (CallFunction|SetDirection))))

(event Input|ActionEvents|InputActionSwordAttack
  (params (Key :type Key%20Structure :default "None"))
  ;[1 1 1] PlayerAttacking
  (:Pressed
    (Game|SpawnActorfromClass "/Game/Sprites/Weapon/DownSwing/S_Sword.S_Sword_C" (Math|Transform|MakeTransform (Transformation|GetWorldLocation (Variables|Default|GetArrow1)) (Math|Rotator|MakeRotator 9e+01 (.roll (Transformation|GetActorRotation)) (+ (.yaw (Math|Rotator|FindLookatRotation (Transformation|GetActorLocation) (.Location (Collision|BreakHitResult (.HitResult (Game|Player|GetHitResultUnderCursorbyChannel (Game|GetPlayerController 0) "TraceTypeQuery1" true)))))) -1.8e+02)) "1,1,1") "Undefined" 0 0)))

(event Input|AxisEvents|InputAxisXAxis
  (params (AxisValue :type Float%20%28single-precision%29))
  ;[1 1 1] Player's Movement
  (Pawn|Input|AddMovementInput (* (Math|Vector|Normalize (+ (Math|Vector|MakeVector 0.0 1.0 0.0) (Math|Vector|MakeVector 1.0 0.0 0.0))) "0,-1.000000, 0") AxisValue true))

(event Input|AxisEvents|InputAxisYAxis
  (params (AxisValue :type Float%20%28single-precision%29))
  ;[1 1 1] Player's Movement
  (Pawn|Input|AddMovementInput "-1.000000,0.000000, 0" AxisValue true))

(event Input|KeyboardEvents|E
  (params (Key :type Key%20Structure :default "None"))
  (bind _returnvalue (Game|GetPlayerController 0))
  (bind _gameinstancereference (Variables|Default|GetGameInstanceReference))
  ;[1 1 1] Pause Menu
  (:Pressed
    (bind _output_get (Variables|/Game/Blueprints/SaveData/BP_SaveGameInstance.BP_SaveGameInstance_C|SetbIsGamePaused _gameinstancereference (not (Variables|/Game/Blueprints/SaveData/BP_SaveGameInstance.BP_SaveGameInstance_C|GetbIsGamePaused _gameinstancereference))))
    (Game|SetGamePaused _output_get)
    (if _output_get
      (bind _returnvalue_2 (UserInterface|CreateWidget "/Game/Widgets/WBP_PauseMenu.WBP_PauseMenu_C"))
      (bind _output_get_2 (Variables|Default|SetPauseMenuReference _returnvalue_2))
      (UserInterface|Viewport|AddtoViewport _output_get_2 0)
      (EventDispatchers|BindEventtoPauseUnpauseEventDispatcher _output_get_2 (delegate Custom|PauseUnpauseGame))
      (Input|SetInputModeGameandUI _returnvalue (Variables|Default|GetPauseMenuReference) "DoNotLock" false)
      (Variables|/Script/Engine.PlayerController|SetbShowMouseCursor _returnvalue true)
      (elif (Utilities|IsValid (Variables|Default|GetPauseMenuReference))
        (Widget|RemovefromParent (Variables|Default|GetPauseMenuReference))
        (Variables|Default|SetPauseMenuReference 0)
        (Input|SetInputModeGameOnly _returnvalue)
        (Variables|/Script/Engine.PlayerController|SetbShowMouseCursor _returnvalue false)))))

(fn ConstructionScript
  (Transformation|SetWorldRotation (Variables|Default|GetSprite) (Math|Rotator|MakeRotator (.pitch (Transformation|GetWorldRotation (Variables|Camera|GetSpringArm))) 0.0 -9e+01) false false))

(fn SetDirection
  ;[1 1 1] Idle Animation
  (if (or (!= (Input|AxisValues|GetXAxis) 0.0) (!= (Input|AxisValues|GetYAxis) 0.0))
    (bind _output_get (Variables|Default|SetDirection (select (and (> (Input|AxisValues|GetXAxis) 0.0) (> (Input|AxisValues|GetYAxis) 0.0)) "NewEnumerator4" (select (and (< (Input|AxisValues|GetXAxis) 0.0) (< (Input|AxisValues|GetYAxis) 0.0)) "NewEnumerator7" (select (and (> (Input|AxisValues|GetXAxis) 0.0) (< (Input|AxisValues|GetYAxis) 0.0)) "NewEnumerator6" (select (and (< (Input|AxisValues|GetXAxis) 0.0) (> (Input|AxisValues|GetYAxis) 0.0)) "NewEnumerator5" (select (> (Input|AxisValues|GetYAxis) 0.0) "NewEnumerator0" (select (< (Input|AxisValues|GetYAxis) 0.0) "NewEnumerator1" (select (> (Input|AxisValues|GetXAxis) 0.0) "NewEnumerator2" "NewEnumerator3")))))))))
    (Utilities|FlowControl|Sequence
      (:then_0
        (Variables|Default|SetCurrentSwing (Utilities|Select :Index _output_get :NewEnumerator0 0 :NewEnumerator1 0 :NewEnumerator2 0 :NewEnumerator3 0 :NewEnumerator4 0 :NewEnumerator5 0 :NewEnumerator6 0 :NewEnumerator7 0)))
      (:then_1
        (if true
          (Sprite|SetFlipbook (Variables|Default|GetSprite) (select (> (Math|Vector|VectorLength (Transformation|GetVelocity)) 0.0) (Utilities|Select :Index (Variables|Default|GetDirection) :NewEnumerator0 "/Game/Sprites/CharacterUpdate/FB_SpriteWalkingUp.FB_SpriteWalkingUp" :NewEnumerator1 "/Game/Sprites/CharacterUpdate/FB_SpriteWalkingDown.FB_SpriteWalkingDown" :NewEnumerator2 "/Game/Sprites/CharacterUpdate/FB_SpriteWalkingRight.FB_SpriteWalkingRight" :NewEnumerator3 "/Game/Sprites/CharacterUpdate/FB_SpriteWalkingLeft.FB_SpriteWalkingLeft" :NewEnumerator4 "/Game/Sprites/CharacterUpdate/FB_SpriteWalkingNorthEast.FB_SpriteWalkingNorthEast" :NewEnumerator5 "/Game/Sprites/CharacterUpdate/FB_SpriteWalkingNWest.FB_SpriteWalkingNWest" :NewEnumerator6 "/Game/Sprites/CharacterUpdate/FB_WalkingSouthEast.FB_WalkingSouthEast" :NewEnumerator7 "/Game/Sprites/CharacterUpdate/FB_SpriteWalkingSouthWest.FB_SpriteWalkingSouthWest") (Utilities|Select :Index (Variables|Default|GetDirection) :NewEnumerator0 "/Game/Sprites/CharacterUpdate/BaseIdle/IdleUp.IdleUp" :NewEnumerator1 "/Game/Sprites/CharacterUpdate/BaseIdle/IdleDown.IdleDown" :NewEnumerator2 "/Game/Sprites/CharacterUpdate/BaseIdle/IdleRight.IdleRight" :NewEnumerator3 "/Game/Sprites/CharacterUpdate/BaseIdle/IdleLeft.IdleLeft" :NewEnumerator4 "/Game/Sprites/CharacterUpdate/BaseIdle/IdleNE.IdleNE" :NewEnumerator5 "/Game/Sprites/CharacterUpdate/BaseIdle/IdleNW.IdleNW" :NewEnumerator6 "/Game/Sprites/CharacterUpdate/BaseIdle/IdleSE.IdleSE" :NewEnumerator7 "/Game/Sprites/CharacterUpdate/BaseIdle/IdleSW.IdleSW")) :!label _label)
          (else
            (Sprite|SetFlipbook (Variables|Default|GetSprite))))))
    (else
      (goto _label))))